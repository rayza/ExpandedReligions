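; BP_AC_BonusStats_Buff is a buff component, apparently a base for buffs that modify bonus stats on the owning character.
; On buff start it runs the parent effect, then fetches and caches the character's BP_ProgressionSystem.
; IncreaseBonusStat and DecreaseBonusStat add or subtract BuffAmount on a stat passed by reference.
; Neither helper is called here, and the tick and cleared events only call their parent.
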(event `self.EffectToApplyOnBuffStart`
  (`parent.EffectToApplyOnBuffStart`)
  (`|ExecutionSequence`
    (:`then_0`
      (bind _returnvalue (`ConanCharacter.GetProgressionSystem` (`self.OwningCharacter`)))
      (bind _asbp_progression_system (cast `/Game/Systems/Progression/BP_ProgressionSystem` _returnvalue))
      (set `self.BP_ProgressionSystem` _asbp_progression_system))))

(event `self.EffectToApplyOnBuffTick`
  (`parent.EffectToApplyOnBuffTick`))

(event `self.EffectToApplyOnBuffCleared`
  (`parent.EffectToApplyOnBuffCleared`))

(fn `DecreaseBonusStat`
  (params (BonusStat :type "Float (double-precision) (by ref)"))
  (`|VariableSetRef` BonusStat (- BonusStat (`self.BuffAmount`))))

(fn `IncreaseBonusStat`
  (params (BonusStat :type "Float (double-precision) (by ref)"))
  (`|VariableSetRef` BonusStat (+ BonusStat (`self.BuffAmount`))))