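; Ishtar buff, likely an actor component, that grants a temporary stat bonus scaled by the Health attribute.
; It extends a parent buff's start and cleared events, calling the parent logic first.
; On start it increases a bonus stat by the progression system's Health attribute; on clear it decreases it by that attribute's value at that moment, with no cached amount.
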(event `self.EffectToApplyOnBuffStart`
  (`parent.EffectToApplyOnBuffStart`)
  (`self.IncreaseBonusStat` (`KismetMathLibrary.Conv_IntToDouble` (`/Game/Systems/Progression/BP_ProgressionSystem.AttributeHealth` (`self.BP_ProgressionSystem`)))))

(event `self.EffectToApplyOnBuffCleared`
  (`parent.EffectToApplyOnBuffCleared`)
  (`self.DecreaseBonusStat` (`KismetMathLibrary.Conv_IntToDouble` (`/Game/Systems/Progression/BP_ProgressionSystem.AttributeHealth` (`self.BP_ProgressionSystem`)))))